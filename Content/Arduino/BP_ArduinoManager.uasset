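; BP_ArduinoManager reads an Arduino sensor over a serial port and plays a weapon-fire sound when the reading falls within a range.
; On BeginPlay it opens the COM port and, if successful, starts a looping timer that reads and prints each line.
; A DoOnce, reset when the value leaves the range, makes the sound play once per entry.
; EndPlay closes the port.
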(event `LeerSensor`
  (bind _serialport (`self.SerialPort`))
  (`/Engine/EditorBlueprintResources/StandardMacros.IsValid` _serialport
    (:`Is Valid`
      (bind (_bsuccess _returnvalue) (`Serial.Readln` _serialport))
      (`KismetSystemLibrary.PrintString` _returnvalue)
      (bind _returnvalue_2 (`KismetStringLibrary.Conv_StringToDouble` _returnvalue))
      (if (and (> _returnvalue_2 1.0) (< _returnvalue_2 20.0))
        (`/Engine/EditorBlueprintResources/StandardMacros.DoOnce` false :!label _label
          (:`Completed`
            (`GameplayStatics.PlaySound2D` "/Game/FPWeapon/Audio/FirstPersonTemplateWeaponFire02.FirstPersonTemplateWeaponFire02" 1.0 1.0 0.0 null null)))
        (else
          (goto _label :!via `Reset`))))))

(event `self.ReceiveBeginPlay`
  (bind (_bopened _returnvalue) (`Serial.OpenComPort` 3))
  (if _bopened
    (set `self.SerialPort` _returnvalue)
    (`KismetSystemLibrary.PrintString` "El puerto se abrio correctamente")
    (`KismetSystemLibrary.K2_SetTimerDelegate` (delegate `LeerSensor`) 0.05 true)
    (else
      (`KismetSystemLibrary.PrintString` "El puerto no se pudo abrir"))))

(event `self.ReceiveEndPlay`
  (params (EndPlayReason :type "EEndPlayReason Enum" :default "Destroyed"))
  (bind _serialport (`self.SerialPort`))
  (`/Engine/EditorBlueprintResources/StandardMacros.IsValid` _serialport
    (:`Is Valid`
      (`Serial.Close` _serialport)
      (`KismetSystemLibrary.PrintString` "Puerto cerrado"))))

(fn `UserConstructionScript`)