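; Player character for a soccer ball juggling (dominadas) game, with mouse look and a kick on F.
; On BeginPlay it shows the HUD and a countdown widget, then enables physics on BP_Balon when the countdown ends.
; HacerDominada plays a kick montage, launches any ball overlapping the ZonaPatada zone upward with a velocity-change impulse, and increments the juggle counter.
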(event `InputAxisKey|MouseX`
  (params (AxisValue :type "Float (single-precision)"))
  (`self.AddControllerYawInput` AxisValue))

(event `InputAxisKey|MouseY`
  (params (AxisValue :type "Float (single-precision)"))
  (`self.AddControllerPitchInput` AxisValue))

(event `Key|F`
  (params (Key :type "Key Structure"))
  (:`Pressed`
    (`self.HacerDominada` self)))

(event `self.ReceiveBeginPlay`
  (bind _textocontador (`/Game/WBP_CuentaRegresiva.TextoContador` (`self.Ref_Contador`)))
  (bind _returnvalue (`|CreateWidget` "/Game/WBP_HUD.WBP_HUD_C"))
  (`UserWidget.AddToViewport` _returnvalue 0)
  (bind _returnvalue_2 (`|CreateWidget` "/Game/WBP_CuentaRegresiva.WBP_CuentaRegresiva_C"))
  (bind _output_get (set `self.Ref_Contador` _returnvalue_2))
  (`UserWidget.AddToViewport` _output_get 0)
  (`KismetSystemLibrary.Delay` 1.0)
  (`TextBlock.SetText` _textocontador "2")
  (`KismetSystemLibrary.Delay` 1.0)
  (`TextBlock.SetText` _textocontador "1")
  (`KismetSystemLibrary.Delay` 1.0)
  (`TextBlock.SetText` _textocontador "go")
  (bind _returnvalue_3 (`GameplayStatics.GetActorOfClass` "/Game/BP_Balon.BP_Balon_C"))
  (`PrimitiveComponent.SetSimulatePhysics` (`/Game/BP_Balon.StaticMesh` _returnvalue_3) true)
  (`Widget.RemoveFromParent` (`self.Ref_Contador`)))

(fn `HacerDominada`
  (`self.PlayAnimMontage` "/Game/AM_AnimacionF.AM_AnimacionF")
  (`KismetSystemLibrary.PrintString` "presione f")
  (for _array_element (`PrimitiveComponent.GetOverlappingActors` (`self.ZonaPatada`) "/Game/BP_Balon.BP_Balon_C")
    (bind _asbp_balon (cast `/Game/BP_Balon` _array_element))
    (`PrimitiveComponent.AddImpulse` (`/Game/BP_Balon.StaticMesh` _asbp_balon) (0.0 0.0 800.0) "None" true)
    (`KismetSystemLibrary.PrintString` "¡SÍ LO TOQUÉ!\".")
    (`/Engine/EditorBlueprintResources/StandardMacros.IncrementInt` (`self.ContadorDominadas`))))

(fn `UserConstructionScript`)